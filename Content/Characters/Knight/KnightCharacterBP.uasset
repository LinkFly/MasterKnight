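; Knight character Blueprint that handles sword-based melee hits against other CustomCharacterBase characters.
; The construction script attaches the sword and its capsule to the right-hand socket and registers that capsule as AttackCapsule.
; During a power attack, capsule overlaps call Attack on any other such character.
; Disconnected experiments remain, including a slow-motion toggle and line-trace hit polling through a local delayed while-loop macro.
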(event OnComponentBeginOverlap(SwordCapsule)
  (params (OverlappedComponent :type Primitive%20Component%20Object%20Reference) (OtherActor :type Actor%20Object%20Reference) (OtherComp :type Primitive%20Component%20Object%20Reference) (OtherBodyIndex :type Integer) (bFromSweep :type Boolean) (SweepResult :type Hit%20Result%20Structure%20%28by%20ref%29))
  (if (Variables|Default|GetIsPowerAttack)
    (bind _ascustom_character_base (Utilities|Casting|CastToCustomCharacterBase OtherActor))
    (if (!= _ascustom_character_base self)
      (Class|CustomCharacterBase|Attack _ascustom_character_base))))

(event EventBeginPlay
  (Variables|Default|SetSwordPredLocation (Transformation|GetWorldLocation (Variables|Default|GetSwordCapsule))))

(event Collision|EventActorBeginOverlap
  (params (OtherActor :type Actor%20Object%20Reference)))

(fn ConstructionScript
  (Transformation|AttachComponentToComponent (Variables|Default|GetSwordCapsule) (Variables|Character|GetMesh) "hand_rSocket" "KeepRelative" "KeepRelative" "KeepRelative" true)
  (Transformation|AttachComponentToComponent (Variables|Default|GetSword) (Variables|Character|GetMesh) "hand_rSocket" "KeepRelative" "KeepRelative" "KeepRelative" true)
  (Variables|/Script/MasterKnight.KnightCharacter|SetAttackCapsule self (Variables|Default|GetSwordCapsule)))