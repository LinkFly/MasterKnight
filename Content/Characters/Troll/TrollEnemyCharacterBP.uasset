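; Troll enemy character Blueprint that sets up hand and body collision capsules on top of inherited character logic.
; The construction script calls the parent, attaches the capsules to hand and pelvis mesh sockets, and assigns the left hand as AttackCapsule.
; The event graph does nothing at runtime: its events are empty, and a leftover chain that attacks non-enemy characters during attacks is disconnected.
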(event OnComponentEndOverlap(LHandCapsule)
  (params (OverlappedComponent :type Primitive%20Component%20Object%20Reference) (OtherActor :type Actor%20Object%20Reference) (OtherComp :type Primitive%20Component%20Object%20Reference) (OtherBodyIndex :type Integer)))

(event EventBeginPlay)

(event Collision|EventActorBeginOverlap
  (params (OtherActor :type Actor%20Object%20Reference)))

(event EventTick
  (params (DeltaSeconds :type Float%20%28single-precision%29)))

(fn ConstructionScript
  (|CallParentFunction)
  (Transformation|AttachComponentToComponent (Variables|Default|GetLHandCapsule) (Variables|Character|GetMesh) "b_MF_Hand_LSocket" "KeepRelative" "KeepRelative" "KeepRelative" true)
  (Transformation|AttachComponentToComponent (Variables|Default|GetRHandCapsule) (Variables|Character|GetMesh) "b_MF_Hand_RSocket" "KeepRelative" "KeepRelative" "KeepRelative" true)
  (Transformation|AttachComponentToComponent (Variables|Default|GetBodyCapsule) (Variables|Character|GetMesh) "b_MF_PelvisSocket" "KeepRelative" "KeepRelative" "KeepRelative" true)
  (Variables|Default|SetAttackCapsule (Variables|Default|GetLHandCapsule)))