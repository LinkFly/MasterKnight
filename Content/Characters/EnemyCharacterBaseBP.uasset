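; Base enemy character that uses EnemyBase_AICon and can turn smoothly to face a target.
; RotateToTarget stores a yaw-only look-at rotation toward the Target actor, falling back to a Blackboard location.
; Tick interpolates toward that rotation until yaw is within tolerance.
; BeginPlay binds OnAllEnemyDeath to trigger YouWin on the custom game instance.
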(event Custom|OnAllEnemyDeath_Event
  (Class|CustomGameInstance|YouWin (stale EventBeginPlay _ascustom_game_instance_bp)))

(event EventBeginPlay
  (bind _ascustom_game_instance_bp (Utilities|Casting|CastToCustomGameInstanceBP (Game|GetGameInstance)))
  (EventDispatchers|AssignOnAllEnemyDeath (delegate Custom|OnAllEnemyDeath_Event)))

(event Collision|EventActorBeginOverlap
  (params (OtherActor :type Actor%20Object%20Reference)))

(event EventTick
  (params (DeltaSeconds :type Float%20%28single-precision%29))
  (if (Variables|Default|GetIsRotating)
    (CallFunction|RotatingtoTarget DeltaSeconds)))

(fn ConstructionScript
  (Variables|Default|SetAIControllerClass "/Game/AI/EnemyBase_AICon.EnemyBase_AICon_C"))

(fn RotatetoTarget
  (params (NewParam :type Boolean))
  (if (not (Variables|Default|GetIsRotating))
    (Variables|Default|SetIsRotating true)
    (bind _newrotation (CallFunction|GetReqRotation))
    (Variables|Default|SetReqRotation _newrotation)))

(fn RotatingtoTarget
  (params (Delta :type Float%20%28single-precision%29))
  (Transformation|SetActorRotation (Math|Interpolation|RInterpTo (Transformation|GetActorRotation) (Variables|Default|GetReqRotation) Delta 3.0))
  (bind _rotated (CallFunction|IsRotated))
  (Variables|Default|SetIsRotating (not _rotated)))

(fn GetTargetLocation
  (bind _target (Variables|Default|GetTarget))
  (if (!= 0 _target)
    (return (Transformation|GetActorLocation _target))
    (else
      (return (AI|Components|Blackboard|GetValueasVector (Variables|/Script/AIModule.AIController|GetBlackboard (AI|GetAIController self)) (Variables|Default|GetLocationKey))))))

(fn GetReqRotation
  (bind _returnvalue (CallFunction|GetTargetLocation))
  (return (Math|Rotator|MakeRotator 0.0 0.0 (.Yaw (Math|Rotator|BreakRotator (Math|Rotator|FindLookatRotation (Transformation|GetActorLocation) _returnvalue))))))

(fn IsRotated
  (return (Math|Float|NearlyEqual(Float) (.Yaw (Math|Rotator|BreakRotator (Variables|Default|GetReqRotation))) (.Yaw (Math|Rotator|BreakRotator (Transformation|GetActorRotation))) 5.0)))

(fn SetRotationDirection
  (bind _returnvalue (Transformation|GetActorRotation))
  (bind _reqrotation (Variables|Default|GetReqRotation))
  (bind _yaw (Math|Rotator|BreakRotator _reqrotation))
  (bind _yaw_2 (Math|Rotator|BreakRotator _returnvalue))
  (if (> _yaw_2 _yaw)
    (return 1)
    (elif (< _yaw_2 _yaw)
      (return -1)
      (else
        (return 0)))))