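; Living water item, a Thing that adds its Life value to the owning character's Life.
; Tick calls Apply as soon as the OwnerCharacter check passes, so the effect needs no separate use action.
; Apply raises the owner's Life, removes the item via DelThing, prints the new total and destroys the actor.
; The construction script sets the item's title and runs the parent's construction script.
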(event EventBeginPlay)

(event Collision|EventActorBeginOverlap
  (params (OtherActor :type Actor%20Object%20Reference)))

(event EventTick
  (params (DeltaSeconds :type Float%20%28single-precision%29))
  (if (!= (Variables|Default|GetOwnerCharacter) 0)
    (Class|ThingBase|Apply)))

(event EventApply
  (bind _ownercharacter (Variables|Default|GetOwnerCharacter))
  (bind _ownercharacter_2 (Variables|Default|GetOwnerCharacter))
  (Variables|/Script/MasterKnight.CustomCharacterBase|SetLife _ownercharacter_2 (+ (Variables|Default|GetLife) (Variables|/Script/MasterKnight.CustomCharacterBase|GetLife _ownercharacter_2)))
  (Class|CustomCharacterBase|DelThing _ownercharacter self)
  (Development|PrintString (Utilities|String|ToString(Integer) (Variables|/Script/MasterKnight.CustomCharacterBase|GetLife _ownercharacter)))
  (Actor|DestroyActor))

(fn ConstructionScript
  (Variables|Default|SetTitle "Living water")
  (|CallParentFunction))