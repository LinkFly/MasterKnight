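; Custom game instance that holds shared game logic: win and game-over messages, interface mode, player life queries and spawning of Things.
; Interface mode shows or hides the HUD inventory, switches mouse cursor and input mode, and optionally pauses the game.
; Things spawn at the world origin from a class or a name looked up in NameClassTable; the CreateThing event stores the result as LastThing.
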(event EventInit)

(event EventYouWin
  (bind _hudwidget (Variables|Default|GetHUDWidget))
  (Variables|/Game/UI/UIHUD.UIHUD_C|SetMainStatusTextValue _hudwidget "Congratilations! You Win!")
  (Default|ShowStartButton _hudwidget))

(event EventGameOver
  (Variables|/Game/UI/UIHUD.UIHUD_C|SetMainStatusTextValue (Variables|Default|GetHUDWidget) "Game Over"))

(event EventCreateThing
  (params (ThingClass :type Thing%20Base%20Class%20Reference))
  (bind _thing (CallFunction|CreateThingbyClass ThingClass))
  (Variables|Default|SetLastThing _thing))

(fn SwitchUsingInterface
  (CallFunction|SetUsingInterface (not (Variables|Default|GetIsUsingInterface))))

(fn EndUsingInterface
  (if (Variables|Default|GetIsGameStarted)
    (CallFunction|SetUsingInterface false)))

(fn StartUsingInterface
  (CallFunction|SetUsingInterface true))

(fn SetUsingInterface
  (params (IsEnable :type Boolean))
  (bind _returnvalue (Game|GetPlayerController 0))
  (bind _output_get (Variables|Default|SetIsUsingInterface IsEnable))
  (if (Variables|Default|GetIsPauseWhenUsingInterface)
    (Game|SetGamePaused _output_get))
  (CallFunction|ShowHIdeInventory _output_get)
  (Variables|/Script/Engine.PlayerController|SetbShowMouseCursor _returnvalue _output_get)
  (if _output_get
    (Input|SetInputModeGameandUI (Game|GetPlayerController 0) 0 "LockAlways" true)
    (else
      (Input|SetInputModeGameOnly _returnvalue))))

(fn ShowHIdeInventory
  (params (IsShow :type Boolean))
  (bind _hudwidget (Variables|Default|GetHUDWidget))
  (bind _menu (Variables|/Game/UI/UIHUD.UIHUD_C|GetMenu _hudwidget))
  (bind _inventory (Variables|/Game/UI/Menu.Menu_C|GetInventory _menu))
  (if IsShow
    (Widget|SetVisibility _inventory "Visible")
    (else
      (Widget|SetVisibility _inventory "Hidden"))))

(fn GetInventory
  (return (Variables|/Game/UI/Menu.Menu_C|GetInventory (Variables|/Game/UI/UIHUD.UIHUD_C|GetMenu (Variables|Default|GetHUDWidget)))))

(fn GetPlayerLife
  (bind _ascustom_character_base (Utilities|Casting|CastToCustomCharacterBase (Game|GetPlayerCharacter 0)))
  (return (Variables|/Script/MasterKnight.CustomCharacterBase|GetLife _ascustom_character_base) (/ (Math|Conversions|ToFloat(Integer) (Variables|/Script/MasterKnight.CustomCharacterBase|GetLife _ascustom_character_base)) (Math|Conversions|ToFloat(Integer) (Variables|CustomGameInstanceBP_C|GetMaxLife self)))))

(fn CreateThingbyClassName
  (params (ClassName :type String))
  (CallFunction|CreateThingbyClass (.Value (Utilities|Map|Find (Variables|Default|GetNameClassTable) ClassName))))

(fn CreateThingbyClass
  (params (ThingClass :type Thing%20Base%20Class%20Reference))
  (if (!= ThingClass 0)
    (bind _returnvalue (Game|SpawnActorfromClass ThingClass (Math|Transform|MakeTransform "0, 0, 0") "Undefined" 0 (Variables|Default|GetPlayerCharacter)))
    (Development|PrintString (Utilities|String|Append "!!! Created: " (Utilities|GetObjectName _returnvalue)))
    (return _returnvalue)))